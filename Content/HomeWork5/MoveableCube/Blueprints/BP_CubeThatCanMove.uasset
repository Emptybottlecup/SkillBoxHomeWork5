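; BP_CubeThatCanMove is a cube pawn that wanders around its spawn point within an X/Y boundary.
; It chains AI MoveTo calls on FloatingPawnMovement, picking a new target whenever a move succeeds or fails.
; Each new target lies 1500 units along a heading toward a random point around the center.
; DoOnce gates let leaving the bounds or hitting something redirect it without repeated triggering.
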(event `self.ReceiveBeginPlay`
  (bind _returnvalue (`self.K2_GetActorLocation`))
  (set `self.Center` _returnvalue)
  (set `self.Target Location` (+ _returnvalue (* (`SceneComponent.GetForwardVector` (`self.Cube`)) 1500)))
  (set `FloatingPawnMovement.MaxSpeed` (`self.Speed`) (`self.FloatingPawnMovement`))
  (`self.Move`))

(event `Move`
  (`|AIMoveTo` self (`self.Target Location`) null
    (:`OnSuccess`
      _)
    (:`OnFail`
      _))
  (`self.ChangeTargetLocation`)
  (`self.Move`))

(event `self.ReceiveTick`
  (params (DeltaSeconds :type "Float (single-precision)"))
  (bind _returnvalue (`self.Pawn In Boundaries`))
  (if _returnvalue
    (goto _label :!via `Reset`)
    (else
      (`/Engine/EditorBlueprintResources/StandardMacros.DoOnce` false :!label _label
        (:`Completed`
          (`self.ChangeTargetLocation`)
          (`self.Move`))))))

(event `self.Cube.OnComponentHit`
  (params (HitComponent :type "PrimitiveComponent Object Reference") (OtherActor :type "Actor Object Reference") (OtherComp :type "PrimitiveComponent Object Reference") (NormalImpulse :type "Vector Structure") (Hit :type "HitResult Structure (by ref)"))
  (`/Engine/EditorBlueprintResources/StandardMacros.DoOnce` false :!label _label_2
    (:`Completed`
      (`self.ChangeTargetLocation`)
      (`self.Move`)
      (`KismetSystemLibrary.Delay` 0.1)
      (goto _label_2 :!via `Reset`))))

(fn `ChangeTargetLocation`
  (`self.K2_SetActorRotation` (`KismetMathLibrary.FindLookAtRotation` (`self.K2_GetActorLocation`) (`KismetMathLibrary.RandomPointInBoundingBox` (`self.Center`) (`KismetMathLibrary.MakeVector` (`self.Max X`) (`self.Max Y`)))))
  (set `self.Target Location` (+ (`self.K2_GetActorLocation` self) (* (`self.GetActorForwardVector` self) 1500))))

(fn `Pawn In Boundaries`
  (returns (ReturnValue :type Boolean))
  (bind (_returnvalue_x _returnvalue_y) (`KismetMathLibrary.BreakVector` (`self.K2_GetActorLocation`)))
  (bind (_center_x _center_y) (`KismetMathLibrary.BreakVector` (`self.Center`)))
  (return (and (`KismetMathLibrary.InRange_FloatFloat` _returnvalue_x (+ _center_x (`self.Min X`)) (+ _center_x (`self.Max X`))) (`KismetMathLibrary.InRange_FloatFloat` _returnvalue_y (+ _center_y (`self.Min Y`)) (+ _center_y (`self.Max Y`))))))

(fn `UserConstructionScript`)